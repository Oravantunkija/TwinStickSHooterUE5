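; EnemyCharacter is a twin-stick shooter enemy that damages the hero on contact and awards score when killed.
; Overlapping a HeroCharacter starts a looping DamageTheHero timer at its attack rate, cleared when that overlap ends.
; AffectHealth handles death by ignoring pawn and dynamic collision, incrementing the GameMode score, detaching the controller and destroying the actor after a delay.
; The construction script tints the body through a dynamic material instance.
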(event `/Game/BluePrints/iDamageable.Affect Health`
  (params (Delta :type "Float (double-precision)"))
  (bind _capsulecomponent (`self.CapsuleComponent`))
  (bind _output_get (set `self.Health` (- (`self.Health`) Delta)))
  (`KismetSystemLibrary.PrintString` (`KismetStringLibrary.Conv_DoubleToString` _output_get))
  (if (<= (`self.Health`) 0.0)
    (set `self.isDead` true)
    (`PrimitiveComponent.SetCollisionResponseToChannel` _capsulecomponent "ECC_WorldDynamic" "ECR_Ignore")
    (`PrimitiveComponent.SetCollisionResponseToChannel` _capsulecomponent "ECC_Pawn" "ECR_Ignore")
    (bind _astwin_shooter_game_mode (cast `/Game/BluePrints/TwinShooterGameMode` (`GameplayStatics.GetGameMode`)))
    (`/Game/BluePrints/TwinShooterGameMode.IncrementScore` _astwin_shooter_game_mode (`self.Score`))
    (`self.DetachFromControllerPendingDestroy`)
    (`KismetSystemLibrary.Delay` 3.0)
    (`self.K2_DestroyActor`)))

(event `self.ReceiveActorBeginOverlap`
  (params (OtherActor :type "Actor Object Reference"))
  (bind _ashero_character (cast `/Game/BluePrints/HeroCharacter` OtherActor))
  (set `self.Hero` _ashero_character)
  (`KismetSystemLibrary.K2_SetTimerDelegate` (delegate `DamageTheHero`) (/ 1.0 (`self.AttacksPerSecond`)) true))

(event `DamageTheHero`
  (if (not (`self.isDead`))
    (`/Game/BluePrints/HeroCharacter.Affect Health` (`self.Hero`) (`self.Damage`))))

(event `self.ReceiveActorEndOverlap`
  (params (OtherActor :type "Actor Object Reference"))
  (if (== OtherActor (`self.Hero`))
    (`KismetSystemLibrary.K2_ClearTimer` null "DamageTheHero")))

(fn `UserConstructionScript`
  (bind _returnvalue (`PrimitiveComponent.CreateDynamicMaterialInstance` (`self.Mesh`) 0 null "None"))
  (bind _output_get (set `self.DynaMat` _returnvalue))
  (`MaterialInstanceDynamic.SetVectorParameterValue` (`self.DynaMat`) "BodyColor" (`self.EnemyColor`))
  (`MaterialInstanceDynamic.SetVectorParameterValue` _output_get "BodyColor" (`self.EnemyColor`)))